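; BP_Beton is a teleporter that moves any actor entering its Box to the linked Portal actor's location with a zeroed rotation.
; Before teleporting, it clears the Portal's Canteleport flag to prevent bouncing back, then calls that Portal's Timer, which re-enables it after one second.
; Leaving the Box calls DoorOpen(false) on Door, restores Canteleport and prints a debug message; the DoorOpen(true) call is unconnected.
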(event OnComponentBeginOverlap(Box)
  (params (OverlappedComponent :type Primitive%20Component%20Object%20Reference) (OtherActor :type Actor%20Object%20Reference) (OtherComp :type Primitive%20Component%20Object%20Reference) (OtherBodyIndex :type Integer) (bFromSweep :type Boolean) (SweepResult :type Hit%20Result%20Structure%20%28by%20ref%29))
  (bind _portal (Variables|Default|GetPortal))
  (if (Variables|Default|Getcanteleport)
    (Variables|BP_Beton_C|Setcanteleport _portal false)
    (Transformation|Teleport OtherActor (Transformation|GetActorLocation _portal) "0, 0, 0")
    (CallFunction|Timer _portal)))

(event OnComponentEndOverlap(Box)
  (params (OverlappedComponent :type Primitive%20Component%20Object%20Reference) (OtherActor :type Actor%20Object%20Reference) (OtherComp :type Primitive%20Component%20Object%20Reference) (OtherBodyIndex :type Integer))
  (Default|DoorOpen (Variables|Default|GetDoor) false)
  (Variables|Default|Setcanteleport true)
  (Development|PrintString (Utilities|String|Append (Utilities|GetDisplayName self) ":end") true true "(R=0.000000,G=0.660000,B=1.000000,A=1.000000)" 999.0))

(event Custom|Timer
  (Utilities|FlowControl|Delay 1.0)
  (Variables|Default|Setcanteleport true))

(fn ConstructionScript)