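; BP_BottomDrawers is a unit of three drawers, each opened and closed by its own toggle event.
; Each event flips an open flag and plays or reverses a timeline that slides the drawer's world location along FirstDrawer's right vector.
; All three drawers offset from a single Start position, captured from FirstDrawer at BeginPlay.
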(event Custom|DRAWERUNO
  (Variables|Default|SetIsFirstDrawerOpen (not (Variables|Default|GetIsFirstDrawerOpen)))
  (if (Variables|Default|GetIsFirstDrawerOpen)
    (bind _newtrack_0 (Timeline|Timeline_0 Play)
      (:Update
        (Transformation|SetWorldLocation (Variables|Default|GetFirstDrawer) (+ (* (Math|Vector|GetRightVector (Variables|Default|GetFirstDrawer)) (* _newtrack_0 3e+01)) (stale EventBeginPlay _output_get)) false false)))
    (else
      (Timeline|Timeline_0 Reverse))))

(event Custom|DRAWERDUO
  (Variables|Default|SetIsSecondDrawerOpen (not (Variables|Default|GetIsSecondDrawerOpen)))
  (if (Variables|Default|GetIsSecondDrawerOpen)
    (bind _newtrack_0 (Timeline|Timeline_1 Play)
      (:Update
        (Transformation|SetWorldLocation (Variables|Default|GetSecondDrawer) (+ (stale EventBeginPlay _output_get) (* (Math|Vector|GetRightVector (Variables|Default|GetFirstDrawer)) (* _newtrack_0 3e+01))) false false)))
    (else
      (Timeline|Timeline_1 Reverse))))

(event Custom|DRAWERTRE
  (Variables|Default|SetIsThirdDrawerOpen (not (Variables|Default|GetIsThirdDrawerOpen)))
  (if (Variables|Default|GetIsThirdDrawerOpen)
    (bind _newtrack_0 (Timeline|Timeline_2 Play)
      (:Update
        (Transformation|SetWorldLocation (Variables|Default|GetThirdDrawer) (+ (* (Math|Vector|GetRightVector (Variables|Default|GetFirstDrawer)) (* _newtrack_0 3e+01)) (stale EventBeginPlay _output_get)) false false)))
    (else
      (Timeline|Timeline_2 Reverse))))

(event EventBeginPlay
  (bind _output_get (Variables|Default|SetStart (Transformation|GetWorldLocation (Variables|Default|GetFirstDrawer)))))

(fn ConstructionScript)