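; Interactive lower cabinet Blueprint with a drawer (Predalcek) and a door (Vratca) that toggle open and closed.
; The PREDAL and VRATA events each flip a boolean, then play or reverse that part's timeline.
; The drawer slides along the actor's right vector from a world position cached at BeginPlay, while the door swings up to 90 degrees in relative yaw.
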(event Custom|PREDAL
  (params (HitComponent :type Primitive%20Component%20Object%20Reference))
  (Variables|Default|SetIsOpenPredal (not (Variables|Default|GetIsOpenPredal)))
  (if (Variables|Default|GetIsOpenPredal)
    (bind _newtrack_0 (Timeline|Timeline_0 Play)
      (:Update
        (Transformation|SetWorldLocation (Variables|Default|Getpredalcek) (+ (stale EventBeginPlay _output_get) (* (Transformation|GetActorRightVector) (* _newtrack_0 3e+01))) false false)))
    (else
      (Timeline|Timeline_0 Reverse))))

(event Custom|VRATA
  (Variables|Default|SetIsOpenOmarica (not (Variables|Default|GetIsOpenOmarica)))
  (if (Variables|Default|GetIsOpenOmarica)
    (bind _newtrack_0 (Timeline|Timeline_1 Play)
      (:Update
        (Transformation|SetRelativeRotation (Variables|Default|GetVratca) (Math|Rotator|MakeRotator 0.0 0.0 (* _newtrack_0 -9e+01)) false false)))
    (else
      (Timeline|Timeline_1 Reverse))))

(event EventBeginPlay
  (bind _output_get (Variables|Default|SetStart (Transformation|GetWorldLocation (Variables|Default|Getpredalcek)))))

(event EventTick
  (params (DeltaSeconds :type Float%20%28single-precision%29)))

(fn ConstructionScript)