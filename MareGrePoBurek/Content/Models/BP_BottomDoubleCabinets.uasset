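; Interactive bottom double cabinet with a sliding drawer and two hinged doors.
; Three custom events each toggle an open flag and play or reverse their own timeline.
; The drawer slides along its right vector from the world location cached at BeginPlay.
; The left and right doors swing in opposite yaw directions through relative rotation.
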(event Custom|CABINETGOSLIDE
  (Variables|Default|SetCabinetDrawerOpen (not (Variables|Default|GetCabinetDrawerOpen)))
  (if (Variables|Default|GetCabinetDrawerOpen)
    (bind _newtrack_0 (Timeline|SLIDEEEE Play)
      (:Update
        (Transformation|SetWorldLocation (Variables|Default|GetCabinetPredal) (+ (* (Math|Vector|GetRightVector (Variables|Default|GetCabinetPredal)) (* _newtrack_0 3e+01)) (stale EventBeginPlay _output_get)) false false)))
    (else
      (Timeline|SLIDEEEE Reverse))))

(event Custom|LEFTGOBR
  (Variables|Default|SetIsLeftOpen (not (Variables|Default|GetIsLeftOpen)))
  (if (Variables|Default|GetIsLeftOpen)
    (bind _newtrack_0 (Timeline|LeftOpen Play)
      (:Update
        (Transformation|SetRelativeRotation (Variables|Default|GetOmarca%20Leva) (Math|Rotator|MakeRotator 0.0 0.0 (* _newtrack_0 9e+01)) false false)))
    (else
      (Timeline|LeftOpen Reverse))))

(event Custom|RIGHTGOBR
  (Variables|Default|SetIsRightOpen (not (Variables|Default|GetIsRightOpen)))
  (if (Variables|Default|GetIsRightOpen)
    (bind _newtrack_0 (Timeline|Timeline_0 Play)
      (:Update
        (Transformation|SetRelativeRotation (Variables|Default|GetOmarcaDesna) (Math|Rotator|MakeRotator 0.0 0.0 (* _newtrack_0 -9e+01)) false false)))
    (else
      (Timeline|Timeline_0 Reverse))))

(event EventBeginPlay
  (bind _output_get (Variables|Default|SetStart (Transformation|GetWorldLocation (Variables|Default|GetCabinetPredal)))))

(fn ConstructionScript)