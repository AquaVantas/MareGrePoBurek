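; Interactive kitchen fridge actor with a swinging door and three sliding drawers.
; Four Slovenian-named custom events each flip an open flag and play or reverse a timeline.
; The door timeline drives relative yaw, while drawer timelines offset world location along the actor's right vector.
; All three drawers share one Start position, cached from the first drawer at BeginPlay, which also sets the door's initial rotation.
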(event Custom|VRATAHLADILNIKA
  (Variables|Default|SetIsFridgeOpen (not (Variables|Default|GetIsFridgeOpen)))
  (if (Variables|Default|GetIsFridgeOpen)
    (bind _newtrack_0 (Timeline|FridgeVrata Play)
      (:Update
        (Transformation|SetRelativeRotation (Variables|Default|GetFridgeDoor) (Math|Rotator|MakeRotator 0.0 0.0 (* _newtrack_0 92.0)) false false)))
    (else
      (Timeline|FridgeVrata Reverse))))

(event Custom|PRVIPREDALHLADILNIKA
  (Variables|Default|SetIsFirstDrawerOpen (not (Variables|Default|GetIsFirstDrawerOpen)))
  (if (Variables|Default|GetIsFirstDrawerOpen)
    (bind _newtrack_0 (Timeline|FridgePrviPredal Play)
      (:Update
        (Transformation|SetWorldLocation (Variables|Default|GetFirstFridgeDrawer) (+ (* (Transformation|GetActorRightVector) (* _newtrack_0 3e+01)) (stale EventBeginPlay _output_get)) false false)))
    (else
      (Timeline|FridgePrviPredal Reverse))))

(event Custom|DRUGIPREDALHLADILNIKA
  (Variables|Default|SetIsSecondDraweOpen (not (Variables|Default|GetIsSecondDraweOpen)))
  (if (Variables|Default|GetIsSecondDraweOpen)
    (bind _newtrack_0 (Timeline|FridgeDrugiPredal Play)
      (:Update
        (Transformation|SetWorldLocation (Variables|Default|GetSecondFridgeDrawer) (+ (* (Transformation|GetActorRightVector) (* _newtrack_0 3e+01)) (stale EventBeginPlay _output_get)) false false)))
    (else
      (Timeline|FridgeDrugiPredal Reverse))))

(event Custom|TRETJIPREDALHLADILNIKA
  (Variables|Default|SetIsTretjiDrawerOpen (not (Variables|Default|GetIsTretjiDrawerOpen)))
  (if (Variables|Default|GetIsTretjiDrawerOpen)
    (bind _newtrack_0 (Timeline|FridgeTretjiPredal Play)
      (:Update
        (Transformation|SetWorldLocation (Variables|Default|GetThirdFridgeDrawer) (+ (* (Transformation|GetActorRightVector) (* _newtrack_0 3e+01)) (stale EventBeginPlay _output_get)) false false)))
    (else
      (Timeline|FridgeTretjiPredal Reverse))))

(event EventBeginPlay
  (Utilities|FlowControl|Sequence
    (:then_0
      (bind _output_get (Variables|Default|SetStart (Transformation|GetWorldLocation (Variables|Default|GetFirstFridgeDrawer)))))
    (:then_1
      (Transformation|SetRelativeRotation (Variables|Default|GetFridgeDoor) "0,-1.000000, 0" false false))))

(fn ConstructionScript)