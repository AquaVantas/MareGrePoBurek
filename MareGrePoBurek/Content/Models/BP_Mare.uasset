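; BP_Mare is a player character with movement, look and jump input that can operate kitchen furniture.
; Interact and Fire share a short debug-drawn line trace from the Sight component, printing the hit component's name.
; The hit actor is cast to the lower cabinet or fridge Blueprint, and the hit component selects which door or drawer function to call.
; An explosion emitter spawn is left unconnected.
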(event Input|ActionEvents|InputActionJump
  (params (Key :type Key%20Structure :default "None"))
  (:Pressed
    (Character|Jump)))

(event Input|ActionEvents|InputActionFire
  (params (Key :type Key%20Structure :default "None"))
  (bind _sight (Variables|Default|GetSight))
  (bind _returnvalue (Transformation|GetWorldLocation _sight))
  (:Pressed
    (bind _outhit (Collision|LineTraceByChannel _returnvalue (+ _returnvalue (* (Math|Vector|GetForwardVector _sight) 4e+02)) "TraceTypeQuery1" false 0 "ForDuration"))
    (Utilities|FlowControl|Sequence
      (:then_0
        (Development|PrintString (Utilities|GetDisplayName (.HitComponent (Collision|BreakHitResult _outhit))))
        (bind _asbp_spodnja_omarica (Utilities|Casting|CastToBP_SpodnjaOmarica (.HitActor (Collision|BreakHitResult _outhit))))
        (if (== (Variables|/Game/Models/BP_SpodnjaOmarica.BP_SpodnjaOmarica_C|GetCabinetDoor1 _asbp_spodnja_omarica) (.HitComponent (Collision|BreakHitResult _outhit)))
          (Default|VRATA _asbp_spodnja_omarica)
          (elif (== (Variables|/Game/Models/BP_SpodnjaOmarica.BP_SpodnjaOmarica_C|Getpredalcek _asbp_spodnja_omarica) (.HitComponent (Collision|BreakHitResult _outhit)))
            (Default|PREDAL _asbp_spodnja_omarica))))
      (:then_1
        (bind _asbp_kitchen_fridge_iguess (Utilities|Casting|CastToBP_KitchenFridgeIGuess (.HitActor (Collision|BreakHitResult _outhit))))
        (if (== (Variables|/Game/Models/BP_KitchenFridgeIGuess.BP_KitchenFridgeIGuess_C|GetHladilnik _asbp_kitchen_fridge_iguess) (.HitComponent (Collision|BreakHitResult _outhit)))
          (Default|VRATAHLADILNIKA _asbp_kitchen_fridge_iguess)
          (elif (== (.HitComponent (Collision|BreakHitResult _outhit)) (Variables|/Game/Models/BP_KitchenFridgeIGuess.BP_KitchenFridgeIGuess_C|GetFirstFridgeDrawer _asbp_kitchen_fridge_iguess))
            (Default|PRVIPREDALHLADILNIKA _asbp_kitchen_fridge_iguess)
            (elif (== (Variables|/Game/Models/BP_KitchenFridgeIGuess.BP_KitchenFridgeIGuess_C|GetSecondFridgeDrawer _asbp_kitchen_fridge_iguess) (.HitComponent (Collision|BreakHitResult _outhit)))
              (Default|DRUGIPREDALHLADILNIKA _asbp_kitchen_fridge_iguess)
              (elif (== (.HitComponent (Collision|BreakHitResult _outhit)) (Variables|/Game/Models/BP_KitchenFridgeIGuess.BP_KitchenFridgeIGuess_C|GetThirdFridgeDrawer _asbp_kitchen_fridge_iguess))
                (Default|TRETJIPREDALHLADILNIKA _asbp_kitchen_fridge_iguess)))))))))

(event Input|ActionEvents|InputActionInterract
  (params (Key :type Key%20Structure :default "None"))
  (bind _sight (Variables|Default|GetSight))
  (bind _returnvalue (Transformation|GetWorldLocation _sight))
  (:Pressed
    (bind _outhit (Collision|LineTraceByChannel _returnvalue (+ _returnvalue (* (Math|Vector|GetForwardVector _sight) 4e+02)) "TraceTypeQuery1" false 0 "ForDuration"))
    (Utilities|FlowControl|Sequence
      (:then_0
        (Development|PrintString (Utilities|GetDisplayName (.HitComponent (Collision|BreakHitResult _outhit))))
        (bind _asbp_spodnja_omarica (Utilities|Casting|CastToBP_SpodnjaOmarica (.HitActor (Collision|BreakHitResult _outhit))))
        (if (== (Variables|/Game/Models/BP_SpodnjaOmarica.BP_SpodnjaOmarica_C|GetCabinetDoor1 _asbp_spodnja_omarica) (.HitComponent (Collision|BreakHitResult _outhit)))
          (Default|VRATA _asbp_spodnja_omarica)
          (elif (== (Variables|/Game/Models/BP_SpodnjaOmarica.BP_SpodnjaOmarica_C|Getpredalcek _asbp_spodnja_omarica) (.HitComponent (Collision|BreakHitResult _outhit)))
            (Default|PREDAL _asbp_spodnja_omarica))))
      (:then_1
        (bind _asbp_kitchen_fridge_iguess (Utilities|Casting|CastToBP_KitchenFridgeIGuess (.HitActor (Collision|BreakHitResult _outhit))))
        (if (== (Variables|/Game/Models/BP_KitchenFridgeIGuess.BP_KitchenFridgeIGuess_C|GetHladilnik _asbp_kitchen_fridge_iguess) (.HitComponent (Collision|BreakHitResult _outhit)))
          (Default|VRATAHLADILNIKA _asbp_kitchen_fridge_iguess)
          (elif (== (.HitComponent (Collision|BreakHitResult _outhit)) (Variables|/Game/Models/BP_KitchenFridgeIGuess.BP_KitchenFridgeIGuess_C|GetFirstFridgeDrawer _asbp_kitchen_fridge_iguess))
            (Default|PRVIPREDALHLADILNIKA _asbp_kitchen_fridge_iguess)
            (elif (== (Variables|/Game/Models/BP_KitchenFridgeIGuess.BP_KitchenFridgeIGuess_C|GetSecondFridgeDrawer _asbp_kitchen_fridge_iguess) (.HitComponent (Collision|BreakHitResult _outhit)))
              (Default|DRUGIPREDALHLADILNIKA _asbp_kitchen_fridge_iguess)
              (elif (== (.HitComponent (Collision|BreakHitResult _outhit)) (Variables|/Game/Models/BP_KitchenFridgeIGuess.BP_KitchenFridgeIGuess_C|GetThirdFridgeDrawer _asbp_kitchen_fridge_iguess))
                (Default|TRETJIPREDALHLADILNIKA _asbp_kitchen_fridge_iguess)))))))))

(event Input|AxisEvents|InputAxisMoveForward
  (params (AxisValue :type Float%20%28single-precision%29))
  (Pawn|Input|AddMovementInput (Math|Rotator|GetRotationXVector (Transformation|GetWorldRotation (Variables|Collision|GetCapsuleComponent))) AxisValue false))

(event Input|AxisEvents|InputAxisMoveRight
  (params (AxisValue :type Float%20%28single-precision%29))
  (Pawn|Input|AddMovementInput (Math|Vector|GetRightVector (Transformation|GetWorldRotation (Variables|Collision|GetCapsuleComponent))) AxisValue false))

(event Input|AxisEvents|InputAxisLookUp
  (params (AxisValue :type Float%20%28single-precision%29))
  (Pawn|Input|AddControllerPitchInput AxisValue))

(event Input|AxisEvents|InputAxisLookRight
  (params (AxisValue :type Float%20%28single-precision%29))
  (Pawn|Input|AddControllerYawInput AxisValue))

(fn ConstructionScript)